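; BP_PlayerCharacter is the player-controlled sprite character, handling world-axis movement and interaction with nearby Interactables.
; BeginPlay adds the Enhanced Input mapping context, and walk actions feed movement input along world X and Y.
; Each tick rotates the sprite to face its X velocity and box-traces around it to cache an interactable whose CanInteract is set.
; The Interact input calls BeginInteraction on that cached target.
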(event `self.ReceiveTick`
  (params (DeltaSeconds :type "Float (single-precision)"))
  (`self.Tick 1`)
  (`self.Tick 2`))

(event `Tick 1`
  (bind _sprite (`self.Sprite`))
  (bind _velocity_x (`KismetMathLibrary.BreakVector` (`MovementComponent.Velocity` (`self.CharacterMovement`))))
  ;[1 1 1] Sprite Flip
  (`self.Update Player Rotation`)
  (`/Engine/EditorBlueprintResources/StandardMacros.CompareFloat` _velocity_x
    (:`>`
      (`SceneComponent.K2_SetRelativeRotation` _sprite (struct :`Yaw` 180.0) false false))
    (:`<`
      (`SceneComponent.K2_SetRelativeRotation` :`self` _sprite))))

(event `EnhancedInput|/Game/Blueprints/Framework/InputActions/IA_FrontWalk`
  (params (ActionValue :type Boolean) (ElapsedSeconds :type "Float (double-precision)") (TriggeredSeconds :type "Float (double-precision)") (InputAction :type "InputAction Object Reference" :default "/Game/Blueprints/Framework/InputActions/IA_FrontWalk.IA_FrontWalk"))
  ;[1 1 1] Movement
  (:`Triggered`
    (`self.AddMovementInput` (0.0 1.0 0.0) (`KismetMathLibrary.Conv_BoolToDouble` ActionValue))))

(event `EnhancedInput|/Game/Blueprints/Framework/InputActions/IA_BackWalking`
  (params (ActionValue :type "Float (double-precision)") (ElapsedSeconds :type "Float (double-precision)") (TriggeredSeconds :type "Float (double-precision)") (InputAction :type "InputAction Object Reference" :default "/Game/Blueprints/Framework/InputActions/IA_BackWalking.IA_BackWalking"))
  ;[1 1 1] Movement
  (:`Triggered`
    (`self.AddMovementInput` (0.0 -1.0 0.0) ActionValue)))

(event `Update Player Rotation`
  ;[1 1 1] Sprite Flip
)

(event `EnhancedInput|/Game/Blueprints/Framework/InputActions/IA_Walking`
  (params (ActionValue :type "Float (double-precision)") (ElapsedSeconds :type "Float (double-precision)") (TriggeredSeconds :type "Float (double-precision)") (InputAction :type "InputAction Object Reference" :default "/Game/Blueprints/Framework/InputActions/IA_Walking.IA_Walking"))
  ;[1 1 1] Movement
  (:`Triggered`
    (`self.AddMovementInput` (1.0 0.0 0.0) ActionValue)))

(event `self.ReceiveBeginPlay`
  (bind _asbp_player_controller (cast `/Game/Blueprints/Framework/BP_PlayerController` (`GameplayStatics.GetPlayerController` 0)))
  (bind _returnvalue (pcsubsystem `EnhancedInputLocalPlayerSubsystem` _asbp_player_controller))
  (`/Engine/EditorBlueprintResources/StandardMacros.IsValid` _returnvalue
    (:`Is Valid`
      (`EnhancedInputSubsystemInterface.AddMappingContext` _returnvalue "/Game/Blueprints/Framework/IMC_PlayerCharacter.IMC_PlayerCharacter" 0 (struct)))))

(event `Tick 2`
  (bind _returnvalue (`SceneComponent.K2_GetComponentLocation` (`self.Sprite`)))
  ;[1 1 1] Box Tracing for Interaction
  (bind _outhit (`KismetSystemLibrary.BoxTraceSingle` (- _returnvalue (30.0 0.0 0.0)) (+ _returnvalue (20.0 20.0 0.0)) (40.0 40.0 40.0) (struct) "TraceTypeQuery1" false (`|MakeArray` (`self.GetOwner`))))
  (bind _asinteractable (cast `/Game/Blueprints/Interactable` (`.HitActor` (`GameplayStatics.BreakHitResult` _outhit)))
    (:`then`
      (if (`/Game/Blueprints/Interactable.CanInteract` _asinteractable)
        (set `self.CurrentInteractable` _asinteractable)
        (else
          (set `self.CurrentInteractable` null :!label _label))))
    (:`CastFailed`
      (goto _label))))

(event `InputAction|Interact`
  (params (Key :type "Key Structure"))
  (bind _currentinteractable (`self.CurrentInteractable`))
  ;[1 1 1] Box Tracing for Interaction
  (:`Pressed`
    (`/Engine/EditorBlueprintResources/StandardMacros.IsValid` _currentinteractable
      (:`Is Valid`
        (`/Game/Blueprints/Interactable.BeginInteraction` _currentinteractable)))))

(fn `UserConstructionScript`)